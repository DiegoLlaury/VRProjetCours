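; Lightning effect actor that periodically flashes two lightning components and plays an audio cue.
; On BeginPlay it starts a looping timer whose interval of a few seconds is randomized once, then fixed for that instance.
; Each strike plays the audio and toggles both components' hidden state in sync through chained delays, giving three progressively shorter flashes.
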(event Custom|LightningAppears
  (Utilities|FlowControl|Sequence
    (:then_0
      (Audio|Components|Audio|Play (Variables|Default|GetAudio) 0.0)
      (Development|SetHiddeninGame (Variables|Default|GetLightning) false false)
      (Utilities|FlowControl|Delay 0.3)
      (Development|SetHiddeninGame (Variables|Default|GetLightning) true false)
      (Utilities|FlowControl|Delay 0.2)
      (Development|SetHiddeninGame (Variables|Default|GetLightning) false false)
      (Utilities|FlowControl|Delay 0.125)
      (Development|SetHiddeninGame (Variables|Default|GetLightning) true false)
      (Utilities|FlowControl|Delay 0.1)
      (Development|SetHiddeninGame (Variables|Default|GetLightning) false false)
      (Utilities|FlowControl|Delay 0.0625)
      (Development|SetHiddeninGame (Variables|Default|GetLightning) true false))
    (:then_1
      (Development|SetHiddeninGame (Variables|Default|GetLightning1) false false)
      (Utilities|FlowControl|Delay 0.3)
      (Development|SetHiddeninGame (Variables|Default|GetLightning1) true false)
      (Utilities|FlowControl|Delay 0.2)
      (Development|SetHiddeninGame (Variables|Default|GetLightning1) false false)
      (Utilities|FlowControl|Delay 0.125)
      (Development|SetHiddeninGame (Variables|Default|GetLightning1) true false)
      (Utilities|FlowControl|Delay 0.1)
      (Development|SetHiddeninGame (Variables|Default|GetLightning1) false false)
      (Utilities|FlowControl|Delay 0.0625)
      (Development|SetHiddeninGame (Variables|Default|GetLightning1) true false))))

(event EventBeginPlay
  (Utilities|Time|SetTimerbyEvent (delegate Custom|LightningAppears) (Math|Random|RandomFloatinRange 4.0 5.0) true))

(fn ConstructionScript)